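; BP_Target is a marker actor that spawns and removes BP_NPC actors.
; BeginPlay caches the actor transform according to the Destroy and Spawn flags, and removes the overlap Box when Destroy is off.
; A Tick timer spawns an NPC at the cached Location every ten seconds, without checking the Spawn flag.
; The Box destroys any BP_NPC that overlaps it.
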(event `self.ReceiveBeginPlay`
  (if (`self.Destroy`)
    (set `self.Location_destroy` (`self.GetTransform`))
    (else
      (`ActorComponent.K2_DestroyComponent` (`self.Box`))))
  (if (`self.Spawn`)
    (set `self.Location` (`self.GetTransform`))))

(event `self.ReceiveTick`
  (params (DeltaSeconds :type "Float (single-precision)"))
  (bind _output_get (set `self.Timer` (+ DeltaSeconds (`self.Timer`))))
  (if (>= _output_get 10.0)
    (`|SpawnActorFromClass` "/Game/Blueprint/BP_NPC.BP_NPC_C" (`self.Location`) "AdjustIfPossibleButAlwaysSpawn" "MultiplyWithRoot" null null)
    (set `self.Timer` 0.0)))

(event `self.Box.OnComponentBeginOverlap`
  (params (OverlappedComponent :type "PrimitiveComponent Object Reference") (OtherActor :type "Actor Object Reference") (OtherComp :type "PrimitiveComponent Object Reference") (OtherBodyIndex :type Integer) (bFromSweep :type Boolean) (SweepResult :type "HitResult Structure (by ref)"))
  (bind _asbp_npc (cast `/Game/Blueprint/BP_NPC` OtherActor))
  (`self.K2_DestroyActor` _asbp_npc))

(fn `UserConstructionScript`)