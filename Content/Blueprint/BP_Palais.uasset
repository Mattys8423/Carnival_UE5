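; BP_Palais is a timed zone that rewards the third-person character with a coin for getting from Enter to Exit quickly.
; Overlapping Enter latches IsEnter before the character cast, then stores the character and shows a new BP_timer widget.
; Overlapping Exit with the character clears the latch, removes the widget, increments Coins if its Timer is under ten seconds, and zeroes the Timer.
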(event `self.Enter.OnComponentBeginOverlap`
  (params (OverlappedComponent :type "PrimitiveComponent Object Reference") (OtherActor :type "Actor Object Reference") (OtherComp :type "PrimitiveComponent Object Reference") (OtherBodyIndex :type Integer) (bFromSweep :type Boolean) (SweepResult :type "HitResult Structure (by ref)"))
  (if (not (`self.Is_enter`))
    (set `self.Is_enter` true)
    (bind _asbp_third_person_character (cast `/Game/ThirdPerson/Blueprints/BP_ThirdPersonCharacter` OtherActor))
    (set `self.As BP Third Person Character` _asbp_third_person_character)
    (bind _returnvalue (`|CreateWidget` "/Game/UI/BP_timer.BP_timer_C"))
    (bind _output_get (set `self.Widget` _returnvalue))
    (`UserWidget.AddToViewport` _output_get 0)))

(event `self.Exit.OnComponentBeginOverlap`
  (params (OverlappedComponent :type "PrimitiveComponent Object Reference") (OtherActor :type "Actor Object Reference") (OtherComp :type "PrimitiveComponent Object Reference") (OtherBodyIndex :type Integer) (bFromSweep :type Boolean) (SweepResult :type "HitResult Structure (by ref)"))
  (cast `/Game/ThirdPerson/Blueprints/BP_ThirdPersonCharacter` OtherActor)
  (set `self.Is_enter` false)
  (`GameViewportSubsystem.RemoveWidget` (subsystem `GameViewportSubsystem`) (`self.Widget`))
  (if (< (`/Game/UI/BP_timer.Timer` (`self.Widget`)) 10.0)
    (`/Engine/EditorBlueprintResources/StandardMacros.IncrementInt` (`/Game/ThirdPerson/Blueprints/BP_ThirdPersonCharacter.Coins` (`self.As BP Third Person Character`))
      (:`  `
        _)))
  (set `/Game/UI/BP_timer.Timer` 0.0 (`self.Widget`)))

(fn `UserConstructionScript`)