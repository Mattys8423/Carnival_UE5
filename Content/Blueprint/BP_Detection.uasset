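; BP_Detection is an actor that counts Can actors entering its Detect_box and flags whether play is under way.
; Each begin overlap by a Can increments the Cans counter, with no decrement on exit.
; Tick sets IsPlaying true whenever the count is above zero.
; The custom End event resets the count to zero, so IsPlaying turns false on a following tick.
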(event `self.ReceiveTick`
  (params (DeltaSeconds :type "Float (single-precision)"))
  (if (> (`self.Cans`) 0)
    (set `self.Is_playing` true)
    (else
      (set `self.Is_playing` false))))

(event `self.detect_box.OnComponentBeginOverlap`
  (params (OverlappedComponent :type "PrimitiveComponent Object Reference") (OtherActor :type "Actor Object Reference") (OtherComp :type "PrimitiveComponent Object Reference") (OtherBodyIndex :type Integer) (bFromSweep :type Boolean) (SweepResult :type "HitResult Structure (by ref)"))
  (cast `/Game/Blueprint/Can` OtherActor)
  (bind _result (`/Engine/EditorBlueprintResources/StandardMacros.IncrementInt` (`self.Cans`))
    (:`  `
      (set `self.Cans` _result))))

(event `End`
  (set `self.Cans` 0))

(fn `UserConstructionScript`)