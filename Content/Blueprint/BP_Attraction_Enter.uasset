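; BP_Attraction_Enter is a paid entrance gate for an attraction, with a door that opens for the third-person character.
; Overlapping the Enter volume, if not already paid, takes one from the character's Bill when above zero, sets IsPaid and teleports the door upward.
; Overlapping the Exit volume returns the door to the position stored at BeginPlay and clears IsPaid, so the next entry must pay again.
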(event `self.ReceiveBeginPlay`
  (set `self.Location` (`SceneComponent.K2_GetComponentLocation` (`self.Door`))))

(event `self.Enter.OnComponentBeginOverlap`
  (params (OverlappedComponent :type "PrimitiveComponent Object Reference") (OtherActor :type "Actor Object Reference") (OtherComp :type "PrimitiveComponent Object Reference") (OtherBodyIndex :type Integer) (bFromSweep :type Boolean) (SweepResult :type "HitResult Structure (by ref)"))
  (bind _bill (`/Game/ThirdPerson/Blueprints/BP_ThirdPersonCharacter.Bill` (`self.As BP Third Person Character`)))
  (bind _asbp_third_person_character (cast `/Game/ThirdPerson/Blueprints/BP_ThirdPersonCharacter` OtherActor))
  (set `self.As BP Third Person Character` _asbp_third_person_character)
  (if (`self.Is_paid`)
    _
    (elif (not (<= _bill 0))
      (`/Engine/EditorBlueprintResources/StandardMacros.DecrementInt` _bill
        (:`  `
          (set `self.Is_paid` true)
          (`SceneComponent.K2_SetWorldLocation` (`self.Door`) (+ (`self.Location`) (0.0 0.0 800.0)) false true))))))

(event `self.Exit.OnComponentBeginOverlap`
  (params (OverlappedComponent :type "PrimitiveComponent Object Reference") (OtherActor :type "Actor Object Reference") (OtherComp :type "PrimitiveComponent Object Reference") (OtherBodyIndex :type Integer) (bFromSweep :type Boolean) (SweepResult :type "HitResult Structure (by ref)"))
  (cast `/Game/ThirdPerson/Blueprints/BP_ThirdPersonCharacter` OtherActor)
  (`SceneComponent.K2_SetWorldLocation` (`self.Door`) (`self.Location`) false true)
  (set `self.Is_paid` false))

(fn `UserConstructionScript`)