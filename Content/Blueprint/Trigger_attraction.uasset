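; Trigger actor that runs a paid can-shooting attraction when the third-person character overlaps it.
; Entry costs a Bill, raises a cube, blends to the booth camera, activates the Shooting component and adds slider, ball-count and crosshair widgets.
; Tick confines the crosshair to a horizontal band until three balls are used, then after a delay End restores the player, awards Coins or Bills from BP_Detection can counts and resets the cans.
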(event `self.ReceiveBeginPlay`
  (set `self.Location_base` (`SceneComponent.K2_GetComponentLocation` (`self.Cube`))))

(event `self.ReceiveActorBeginOverlap`
  (params (OtherActor :type "Actor Object Reference"))
  (bind _my_third_person_character (`self.My_third_person_character`))
  (bind _my_third_person_character_2 (`self.My_third_person_character`))
  (bind _returnvalue (`self.GetComponentByClass` (`self.My_third_person_character`) "/Game/ThirdPerson/Blueprints/Shooting.Shooting_C"))
  (bind _bill (`/Game/ThirdPerson/Blueprints/BP_ThirdPersonCharacter.Bill` _my_third_person_character_2))
  (bind _asbp_third_person_character (cast `/Game/ThirdPerson/Blueprints/BP_ThirdPersonCharacter` OtherActor))
  (set `self.My_third_person_character` _asbp_third_person_character)
  (`ActorComponent.SetActive` (`self.GetComponentByClass` _my_third_person_character_2 "/Script/Engine.CharacterMovementComponent") false false)
  (if (<= _bill 0)
    (`ActorComponent.SetActive` (`self.GetComponentByClass` (`self.My_third_person_character`) "/Script/Engine.CharacterMovementComponent") true false)
    (else
      (`/Engine/EditorBlueprintResources/StandardMacros.DecrementInt` _bill
        (:`  `
          (`SceneComponent.K2_SetWorldLocation` (`self.Cube`) (+ (`self.Location_base`) (0.0 0.0 800.0)) false true)
          (`KismetSystemLibrary.Delay` 0.2)
          (set `/Game/ThirdPerson/Blueprints/BP_ThirdPersonCharacter.Is_in_Attraction` true _my_third_person_character)
          (`/Game/ThirdPerson/Blueprints/BP_ThirdPersonCharacter.Widget_activate` _my_third_person_character)
          (`PlayerController.SetViewTargetWithBlend` (`GameplayStatics.GetPlayerController` 0) (`ActorComponent.GetOwner` (`self.Camera`)) 1.0 "VTBlend_Linear" 0.0 false)
          (set `/Game/ThirdPerson/Blueprints/Shooting.Camera_attraction` (`self.Camera`) _returnvalue)
          (`ActorComponent.SetActive` _returnvalue true false)
          (bind _returnvalue_2 (`|CreateWidget` "/Game/UI/Slider_CT.Slider_CT_C"))
          (bind _output_get (set `self.Slider_widget` _returnvalue_2))
          (`UserWidget.AddToViewport` _output_get 0)
          (bind _returnvalue_3 (`|CreateWidget` "/Game/UI/Number_ball.Number_ball_C"))
          (bind _output_get_2 (set `self.Nb_ball_widget` _returnvalue_3))
          (`UserWidget.AddToViewport` _output_get_2 0)
          (bind _returnvalue_4 (`|CreateWidget` "/Game/UI/Crosshair.Crosshair_C"))
          (bind _output_get_3 (set `self.Crosshair` _returnvalue_4))
          (`UserWidget.AddToViewport` _output_get_3 0)
          (set `self.Crosshair Img` (`/Game/UI/Crosshair.Crosshair_img` _returnvalue_4))
          (set `self.Ready` true))))))

(event `self.ReceiveTick`
  (params (DeltaSeconds :type "Float (single-precision)"))
  (bind _returnvalue (`KismetMathLibrary.FClamp` (`PlayerController.GetMousePosition` (`GameplayStatics.GetPlayerController` 0)) 475.0 750.0))
  (if (`self.Ready`)
    (if (> (`KismetMathLibrary.Abs` (`KismetMathLibrary.BreakVector2D` (- (/ (`WidgetLayoutLibrary.GetViewportSize`) (2.0 2.0)) (`KismetMathLibrary.MakeVector2D` (`PlayerController.GetMousePosition` (`GameplayStatics.GetPlayerController` 0)) 550.0)))) 200.0)
      (`PlayerController.SetMouseLocation` (`GameplayStatics.GetPlayerController` 0) (`KismetMathLibrary.FTrunc` _returnvalue) 550))
    (`CanvasPanelSlot.SetPosition` (`WidgetLayoutLibrary.SlotAsCanvasSlot` (`self.Crosshair Img`)) (`SlateBlueprintLibrary.ScreenToViewport` (`KismetMathLibrary.MakeVector2D` _returnvalue 550.0)))
    (if (>= (`/Game/ThirdPerson/Blueprints/Shooting.Number_ball` (`self.GetComponentByClass` (`GameplayStatics.GetPlayerPawn` 0) "/Game/ThirdPerson/Blueprints/Shooting.Shooting_C")) 3.0)
      (`ActorComponent.SetActive` (`self.GetComponentByClass` (`self.My_third_person_character`) "/Game/ThirdPerson/Blueprints/Shooting.Shooting_C") false false)
      (`KismetSystemLibrary.Delay` 3.0)
      (`self.End`))))

(event `End`
  (bind _my_third_person_character (`self.My_third_person_character`))
  (`PlayerController.SetViewTargetWithBlend` (`GameplayStatics.GetPlayerController` 0) (`ActorComponent.GetOwner` (`self.GetComponentByClass` (`self.My_third_person_character`) "/Script/Engine.CameraComponent")) 1.0 "VTBlend_Linear" 0.0 false)
  (`ActorComponent.SetActive` (`self.GetComponentByClass` (`self.My_third_person_character`) "/Script/Engine.CharacterMovementComponent") true false)
  (`WidgetLayoutLibrary.RemoveAllWidgets`)
  (`/Game/ThirdPerson/Blueprints/Shooting.Reinit_ball` (`self.GetComponentByClass` (`self.My_third_person_character`) "/Game/ThirdPerson/Blueprints/Shooting.Shooting_C"))
  (set `/Game/ThirdPerson/Blueprints/BP_ThirdPersonCharacter.Is_in_Attraction` false _my_third_person_character)
  (`/Game/ThirdPerson/Blueprints/BP_ThirdPersonCharacter.Widget_activate` _my_third_person_character)
  (bind _outactors (`GameplayStatics.GetAllActorsOfClass` "/Game/Blueprint/BP_Detection.BP_Detection_C"))
  (for _array_element _outactors
    (bind _output_get (set `self.BP_detect` _array_element))
    (if (`/Game/Blueprint/BP_Detection.Is_playing` _output_get)
      (bind _cans (`/Game/Blueprint/BP_Detection.Cans` _output_get))
      (if (>= _cans 8)
        (`/Engine/EditorBlueprintResources/StandardMacros.IncrementInt` (`/Game/ThirdPerson/Blueprints/BP_ThirdPersonCharacter.Coins` (`self.My_third_person_character`))
          (:`  `
            _)))
      (if (== _cans 15)
        (`/Engine/EditorBlueprintResources/StandardMacros.IncrementInt` (`/Game/ThirdPerson/Blueprints/BP_ThirdPersonCharacter.Bill` (`self.My_third_person_character`))
          (:`  `
            _)))
      (`/Game/Blueprint/BP_Detection.End` (`self.BP_detect`))
      (bind _outactors_2 (`GameplayStatics.GetAllActorsOfClass` "/Game/Blueprint/Can.Can_C"))
      (for _array_element_2 _outactors_2
        (`/Game/Blueprint/Can.Reinit` _array_element_2)
        (`SceneComponent.K2_SetWorldLocation` (`self.Cube`) (`self.Location_base`) false true)))))

(fn `UserConstructionScript`)