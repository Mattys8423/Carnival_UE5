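; BP_NPC is a wandering NPC that moves between randomly chosen BP_Target actors in the level.
; BeginPlay caches the targets and calls Move, which sends the pawn to one of them with AIMoveTo; landing also calls Move.
; Tick, gated by a delay, detects zero velocity and triggers the end-move step, which waits a random few seconds before moving again.
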(event `self.OnLanded`
  (params (Hit :type "HitResult Structure (by ref)"))
  (`self.Move`))

(event `self.ReceiveBeginPlay`
  (bind _outactors (`GameplayStatics.GetAllActorsOfClass` "/Game/Blueprint/BP_Target.BP_Target_C"))
  (set `self.Out Actors` _outactors)
  (`self.Move`))

(event `Move`
  (set `self.Arrived` false)
  (`|AIMoveTo` self (0.0 0.0 0.0) (`KismetArrayLibrary.Array_Random` (`self.Out Actors`)) 100.0))

(event `End_Move`
  (`KismetSystemLibrary.Delay` (`KismetMathLibrary.RandomFloatInRange` 2.0 6.0))
  (`self.Move`))

(event `self.ReceiveTick`
  (params (DeltaSeconds :type "Float (single-precision)"))
  (`KismetSystemLibrary.Delay` 2.0)
  (if (== (`self.GetVelocity`) (0.0 0.0 0.0))
    (`self.End_Move`)))

(fn `UserConstructionScript`)