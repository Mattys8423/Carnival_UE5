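; BP_Score is a scoreboard actor for a football game, showing red and blue team scores on two text renders.
; Red_Goal and Blue_Goal events increment a score and refresh its text.
; When a BP_ThirdPersonCharacter hits the Cylinder, it acts as a reset button, zeroing and redisplaying both scores.
; The Cylinder shifts slightly, returns to its saved location after a delay, then BP_Football is reinitialized.
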(event `self.ReceiveBeginPlay`
  (set `self.location_base` (`SceneComponent.K2_GetComponentLocation` (`self.Cylinder`))))

(event `Show`
  (`TextRenderComponent.K2_SetText` (`self.TextRender1`) (`KismetTextLibrary.Conv_IntToText` (`self.Score_red`)))
  (`TextRenderComponent.K2_SetText` (`self.TextRender`) (`KismetTextLibrary.Conv_IntToText` (`self.Score_blue`))))

(event `Red_Goal`
  (bind _score_red (`self.Score_red`))
  (`/Engine/EditorBlueprintResources/StandardMacros.IncrementInt` _score_red
    (:`  `
      (`TextRenderComponent.K2_SetText` (`self.TextRender1`) (`KismetTextLibrary.Conv_IntToText` _score_red)))))

(event `Blue_Goal`
  (bind _score_blue (`self.Score_blue`))
  (`/Engine/EditorBlueprintResources/StandardMacros.IncrementInt` _score_blue
    (:`  `
      (`TextRenderComponent.K2_SetText` (`self.TextRender`) (`KismetTextLibrary.Conv_IntToText` _score_blue)))))

(event `self.Cylinder.OnComponentHit`
  (params (HitComponent :type "PrimitiveComponent Object Reference") (OtherActor :type "Actor Object Reference") (OtherComp :type "PrimitiveComponent Object Reference") (NormalImpulse :type "Vector Structure") (Hit :type "HitResult Structure (by ref)"))
  (cast `/Game/ThirdPerson/Blueprints/BP_ThirdPersonCharacter` OtherActor)
  (set `self.Score_red` 0)
  (set `self.Score_blue` 0)
  (`self.Show`)
  (`self.button`))

(event `button`
  (`SceneComponent.K2_SetWorldLocation` (`self.Cylinder`) (+ (`SceneComponent.K2_GetComponentLocation` (`self.Cylinder`)) (1.0 0.0 0.0)) false true)
  (`KismetSystemLibrary.Delay` 1.0)
  (`SceneComponent.K2_SetWorldLocation` (`self.Cylinder`) (`self.location_base`) false true)
  (bind _returnvalue (`GameplayStatics.GetActorOfClass` "/Game/Blueprint/BP_Football.BP_Football_C"))
  (`/Game/Blueprint/BP_Football.reinit` _returnvalue))

(fn `UserConstructionScript`)