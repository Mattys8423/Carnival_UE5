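; Can is a physics-driven cylinder actor that can be reset to its starting placement.
; BeginPlay stores the cylinder's world transform.
; The Reinit event switches off physics simulation, teleports the cylinder back to that transform without sweeping, then switches simulation back on.
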(event `self.ReceiveBeginPlay`
  (set `self.Initialtransform` (`SceneComponent.K2_GetComponentToWorld` (`self.Cylinder`))))

(event `Reinit`
  (`PrimitiveComponent.SetSimulatePhysics` (`self.Cylinder`) false)
  (`SceneComponent.K2_SetWorldTransform` (`self.Cylinder`) (`self.Initialtransform`) false true)
  (`PrimitiveComponent.SetSimulatePhysics` (`self.Cylinder`) true))

(event `self.ReceiveTick`
  (params (DeltaSeconds :type "Float (single-precision)")))

(fn `UserConstructionScript`)