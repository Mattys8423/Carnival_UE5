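; Goal is a trigger actor that detects when the football enters a goal and scores it.
; On Box overlap with a BP_Football, it branches on the IsRed flag.
; It calls RedGoal or BlueGoal on the BP_Score actor found via GetActorOfClass, then calls Reinit on the football.
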(event `self.Box.OnComponentBeginOverlap`
  (params (OverlappedComponent :type "PrimitiveComponent Object Reference") (OtherActor :type "Actor Object Reference") (OtherComp :type "PrimitiveComponent Object Reference") (OtherBodyIndex :type Integer) (bFromSweep :type Boolean) (SweepResult :type "HitResult Structure (by ref)"))
  (bind _asbp_football (cast `/Game/Blueprint/BP_Football` OtherActor))
  (set `self.As BP Football` _asbp_football)
  (if (`self.Is_Red`)
    (bind _returnvalue (`GameplayStatics.GetActorOfClass` "/Game/Blueprint/BP_Score.BP_Score_C"))
    (`/Game/Blueprint/BP_Score.Red_Goal` _returnvalue)
    (`/Game/Blueprint/BP_Football.reinit` (`self.As BP Football`))
    (else
      (bind _returnvalue_2 (`GameplayStatics.GetActorOfClass` "/Game/Blueprint/BP_Score.BP_Score_C"))
      (`/Game/Blueprint/BP_Score.Blue_Goal` _returnvalue_2)
      (`/Game/Blueprint/BP_Football.reinit` (`self.As BP Football`)))))

(fn `UserConstructionScript`)