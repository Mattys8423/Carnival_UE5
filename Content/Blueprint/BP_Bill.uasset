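; BP_Bill is an actor that opens a BP_Bill_widget screen when the third-person character enters its Box trigger.
; On overlap it deactivates the character's movement component, sets IsModal, marks itself active and shows the mouse cursor.
; The Back_Game event removes the widget, hides the cursor, clears IsModal and reactivates movement, but leaves IsActive set.
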(event `self.Box.OnComponentBeginOverlap`
  (params (OverlappedComponent :type "PrimitiveComponent Object Reference") (OtherActor :type "Actor Object Reference") (OtherComp :type "PrimitiveComponent Object Reference") (OtherBodyIndex :type Integer) (bFromSweep :type Boolean) (SweepResult :type "HitResult Structure (by ref)"))
  (bind _as_bp_third_person_character (`self.As BP Third Person Character`))
  (bind _asbp_third_person_character (cast `/Game/ThirdPerson/Blueprints/BP_ThirdPersonCharacter` OtherActor))
  (set `self.As BP Third Person Character` _asbp_third_person_character)
  (`ActorComponent.SetActive` (`self.GetComponentByClass` _as_bp_third_person_character "/Script/Engine.CharacterMovementComponent") false false)
  (set `/Game/ThirdPerson/Blueprints/BP_ThirdPersonCharacter.Is_modal` true _as_bp_third_person_character)
  (set `self.Is_active` true)
  (bind _returnvalue (`|CreateWidget` "/Game/UI/BP_Bill_widget.BP_Bill_widget_C"))
  (bind _output_get (set `self.Widget` _returnvalue))
  (`UserWidget.AddToViewport` _output_get 0)
  (set `PlayerController.bShowMouseCursor` true (`GameplayStatics.GetPlayerController` 0)))

(event `Back_Game`
  (bind _as_bp_third_person_character (`self.As BP Third Person Character`))
  (`GameViewportSubsystem.RemoveWidget` (subsystem `GameViewportSubsystem`) (`self.Widget`))
  (set `PlayerController.bShowMouseCursor` false (`GameplayStatics.GetPlayerController` 0))
  (set `/Game/ThirdPerson/Blueprints/BP_ThirdPersonCharacter.Is_modal` false _as_bp_third_person_character)
  (`ActorComponent.SetActive` (`self.GetComponentByClass` _as_bp_third_person_character "/Script/Engine.CharacterMovementComponent") true false))

(fn `UserConstructionScript`)