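; BP_Football is a physics football that the third-person character kicks by running into it.
; A hit from BP_ThirdPersonCharacter stores that character and opens a 0.2-second window in which Tick applies an impulse every frame along the character's forward vector.
; The sphere's starting transform is saved on BeginPlay, and the reinit event teleports it back there, toggling physics simulation off and on around the move.
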(event `self.ReceiveBeginPlay`
  (set `self.transform` (`SceneComponent.K2_GetComponentToWorld` (`self.Sphere`))))

(event `self.ReceiveTick`
  (params (DeltaSeconds :type "Float (single-precision)"))
  (if (`self.Can_Shoot`)
    (`PrimitiveComponent.AddImpulse` (`self.Sphere`) (* (`self.GetActorForwardVector` (`self.As BP Third Person Character`)) (`self.Impulse`)) "None" false)))

(event `self.Sphere.OnComponentHit`
  (params (HitComponent :type "PrimitiveComponent Object Reference") (OtherActor :type "Actor Object Reference") (OtherComp :type "PrimitiveComponent Object Reference") (NormalImpulse :type "Vector Structure") (Hit :type "HitResult Structure (by ref)"))
  (bind _asbp_third_person_character (cast `/Game/ThirdPerson/Blueprints/BP_ThirdPersonCharacter` OtherActor))
  (set `self.As BP Third Person Character` _asbp_third_person_character)
  (set `self.Can_Shoot` true)
  (`KismetSystemLibrary.Delay` 0.2)
  (set `self.Can_Shoot` false))

(event `reinit`
  (`PrimitiveComponent.SetSimulatePhysics` (`self.Sphere`) false)
  (`SceneComponent.K2_SetWorldTransform` (`self.Sphere`) (`self.transform`) false true)
  (`PrimitiveComponent.SetSimulatePhysics` (`self.Sphere`) true))

(fn `UserConstructionScript`)